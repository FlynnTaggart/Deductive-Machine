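; Enemy projectile actor that damages pawns on hit and destroys itself upon striking anything other than its owner.
; Health loss is the victim's HealthPoints divided by its ShotsToBeKilled, written directly to CurrentHealthPoints rather than through Unreal's damage system.
; AI health lives on the AIC_Base controller, with no death check here.
; BP_VRCharacter holds its own health, gets a debug print, and has Death called at zero or below.
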(event `self.ReceiveHit`
  (params (MyComp :type "PrimitiveComponent Object Reference") (Other :type "Actor Object Reference") (OtherComp :type "PrimitiveComponent Object Reference") (bSelfMoved :type Boolean) (HitLocation :type "Vector Structure") (HitNormal :type "Vector Structure") (NormalImpulse :type "Vector Structure") (Hit :type "HitResult Structure (by ref)"))
  (if (!= Other (`self.GetOwner`))
    (bind _aspawn (cast `Pawn` Other)
      (:`then`
        (bind _returnvalue (`Pawn.GetController` _aspawn))
        (bind _asaic_base (cast `/Game/Code/AI/Brain/AIC_Base` _returnvalue)
          (:`then`
            (set `/Game/Code/AI/Brain/AIC_Base.CurrentHealthPoints` (- (`/Game/Code/AI/Brain/AIC_Base.CurrentHealthPoints` _asaic_base) (/ (`/Game/Code/AI/Brain/AIC_Base.HealthPoints` _asaic_base) (`/Game/Code/AI/Brain/AIC_Base.ShotsToBeKilled` _asaic_base))) _asaic_base))
          (:`CastFailed`
            (bind _asbp_vrcharacter (cast `/Game/Code/Core/Player/BP_VRCharacter` (`Controller.K2_GetPawn` _returnvalue))
              (:`then`
                (`KismetSystemLibrary.PrintString` "Hello")
                (bind _output_get (set `/Game/Code/Core/Player/BP_VRCharacter.CurrentHealthPoints` (- (`/Game/Code/Core/Player/BP_VRCharacter.CurrentHealthPoints` _asbp_vrcharacter) (/ (`/Game/Code/Core/Player/BP_VRCharacter.HealthPoints` _asbp_vrcharacter) (`/Game/Code/Core/Player/BP_VRCharacter.ShotsToBeKilled` _asbp_vrcharacter))) _asbp_vrcharacter))
                (if (<= _output_get 0.0)
                  (`/Game/Code/Core/Player/BP_VRCharacter.Death` _asbp_vrcharacter)))
              (:`CastFailed`
                _)))))
      (:`CastFailed`
        _))
    (`self.K2_DestroyActor`)))

(fn `UserConstructionScript`)