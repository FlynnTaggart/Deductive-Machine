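; BP_PlayerController is a player controller that turns axis input into smooth locomotion for the VR character.
; On BeginPlay it casts and caches the player character as BP_VRCharacter.
; Move_Y moves the character forward or back along the control rotation's yaw only, scaled by MoveSpeed.
; Move_X turns it continuously through yaw input scaled by RotateRate, with both axes ignoring input inside a dead zone.
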(event `self.ReceiveBeginPlay`
  (bind _asbp_vrcharacter (cast `/Game/Code/Core/Player/BP_VRCharacter` (`GameplayStatics.GetPlayerCharacter` 0)))
  (set `self.PlayerCharacterRef` _asbp_vrcharacter))

(event `InputAxis|Move_Y`
  (params (AxisValue :type "Float (single-precision)"))
  (bind _playercharacterref (`self.PlayerCharacterRef`))
  (bind (_returnvalue_roll _returnvalue_pitch _returnvalue_yaw) (`KismetMathLibrary.BreakRotator` (`Pawn.GetControlRotation` _playercharacterref)))
  (if (> (`KismetMathLibrary.Abs` AxisValue) 0.3)
    (`Pawn.AddMovementInput` _playercharacterref (`KismetMathLibrary.GetForwardVector` (`KismetMathLibrary.MakeRotator` 0.0 0.0 _returnvalue_yaw)) (* AxisValue (`self.MoveSpeed`)) false)))

(event `InputAxis|Move_X`
  (params (AxisValue :type "Float (single-precision)"))
  (if (> (`KismetMathLibrary.Abs` AxisValue) 0.3)
    (`Pawn.AddControllerYawInput` (`self.PlayerCharacterRef`) (* AxisValue (`self.RotateRate`)))))

(fn `UserConstructionScript`)