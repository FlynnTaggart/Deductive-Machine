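; VR player character with physics-simulated hands that can grab physics objects and toggle a hand tablet's message.
; Constraints bind each simulated hand mesh to a non-physical mesh at BeginPlay.
; Grab input sphere-traces from that hand and constrains any simulating hit component to it, breaking the constraint on release.
; Right-hand grab state and grip axis feed animation through casts to two different AnimBP classes, ABP_Hand and ABP_RoboHand.
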(event `self.ReceiveTick`
  (params (DeltaSeconds :type "Float (single-precision)"))
  (if (`self.IsClenchedRight`)
    (set `self.GripStateRight` "NewEnumerator2")
    (else
      (set `self.GripStateRight` "NewEnumerator0")))
  (bind _asabp_hand (cast `/Game/Code/Core/Player/ABP_Hand` (`SkeletalMeshComponent.GetAnimInstance` (`self.SM_Right`))))
  (set `/Game/Code/Core/Player/ABP_Hand.GripState` (`self.GripStateRight`) _asabp_hand))

(event `InputAction|GrabRight`
  (params (Key :type "Key Structure"))
  (:`Pressed`
    (set `self.IsClenchedRight` true))
  (:`Released`
    (set `self.IsClenchedRight` false)))

(event `InputAction|ShowTablet`
  (params (Key :type "Key Structure"))
  (:`Pressed`
    (message `/Game/Code/Core/Interfaces/BPI_HandTablet.ToggleTablet` (`ChildActorComponent.ChildActor` (`self.HandTablet`)))))

(event `self.ReceiveBeginPlay`
  (`PhysicsConstraintComponent.SetConstrainedComponents` (`self.PhysConstraint_Right`) (`self.NonPhysMesh_Right`) "None" (`self.SM_Right`) "Root")
  (`PhysicsConstraintComponent.SetConstrainedComponents` (`self.PhysConstraint_Left`) (`self.NonPhysMesh_Left`) "None" (`self.SM_Left`) "None")
  (`PrimitiveComponent.SetSimulatePhysics` (`self.SM_Right`) true)
  (`PrimitiveComponent.SetSimulatePhysics` (`self.SM_Left`) true))

(event `InputAction|GrabLeft`
  (params (Key :type "Key Structure"))
  (:`Pressed`
    (`self.Grab` false))
  (:`Released`
    (`PhysicsConstraintComponent.BreakConstraint` (`self.GrabConstraint_Left`))))

(event `InputAction|GrabRight`
  (params (Key :type "Key Structure"))
  (:`Pressed`
    (`self.Grab` true))
  (:`Released`
    (`PhysicsConstraintComponent.BreakConstraint` (`self.GrabConstraint_Right`))))

(event `InputAxis|GripRight`
  (params (AxisValue :type "Float (single-precision)"))
  (bind _asabp_robo_hand (cast `/Game/RawContent/Animations/RoboHand/ABP_RoboHand` (`SkeletalMeshComponent.GetAnimInstance` (`self.SM_Right`))))
  (set `/Game/RawContent/Animations/RoboHand/ABP_RoboHand.Grip` AxisValue _asabp_robo_hand))

(fn `Grab`
  (params (bRight :type Boolean))
  (locals (bRightArm :type Boolean))
  (bind _brightarm (`local.bRightArm`))
  (bind _returnvalue (select `bool` (`local.bRightArm`) :`false` (`self.HeldObjectLocationLeft`) :`true` (`self.HeldObjectLocationRight`)))
  (bind _returnvalue_2 (`SceneComponent.K2_GetComponentLocation` _returnvalue))
  (set `local.bRightArm` bRight)
  (bind (_outhit _returnvalue_3) (`KismetSystemLibrary.SphereTraceSingleForObjects` :`Start` _returnvalue_2 :`End` (`/Game/Code/Core/FunctionLibrary/BPML_VectorAlgebra.AddScaledDirection` _returnvalue_2 (`KismetMathLibrary.GetForwardVector` (`SceneComponent.K2_GetComponentRotation` _returnvalue)) 3.0) :`Radius` 4.0 :`ObjectTypes` (`|MakeArray` "ObjectTypeQuery4" :!type "EObjectTypeQuery Enum") :`DrawDebugType` "ForDuration"))
  (if _returnvalue_3
    (bind (_bblockinghit _binitialoverlap _time _distance _location _impactpoint _normal _impactnormal _physmat _hitactor _hitcomponent) (`GameplayStatics.BreakHitResult` _outhit))
    (if (`SceneComponent.IsSimulatingPhysics` _hitcomponent "None")
      (`PhysicsConstraintComponent.SetConstrainedComponents` (select `bool` _brightarm :`false` (`self.GrabConstraint_Left`) :`true` (`self.GrabConstraint_Right`)) (select `bool` _brightarm :`false` (`self.SM_Left`) :`true` (`self.SM_Right`)) "None" _hitcomponent "Root"))))

(fn `UserConstructionScript`)