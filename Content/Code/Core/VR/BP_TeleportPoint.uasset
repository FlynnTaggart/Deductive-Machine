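; Teleport point actor that moves the player to its paired point and swaps streamed levels between the two.
; On BeginPlay it searches the TeleportManager's pairs for itself, caching its partner and both stream level names.
; Player overlap starts a non-blocking load of the partner's level and teleports the player to an offset from the partner, using its rotation combined with a 180-degree turn.
; Ending the overlap unloads this point's level.
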(event `self.ReceiveBeginPlay`
  (for _array_element (`/Game/Code/Core/VR/BP_TeleportManager.TeleportPairs` (`self.TeleportManager`))
    (if (== (break `/Game/Code/Core/Structs/STeleportPointPair` _array_element) self)
      (set `self.StreamNameThis` (`.FirstStramName_12_130BD56F47F345A8F33F9DB0E82DF619` (break `/Game/Code/Core/Structs/STeleportPointPair` _array_element)))
      (set `self.StreamNameOther` (`.SecondStreamName_13_FC1ED26F4C2318AF77202B8F3E32B5BD` (break `/Game/Code/Core/Structs/STeleportPointPair` _array_element)))
      (set `self.OtherPoint` (`.Second_5_44C94781437593443EC271BAB9188421` (break `/Game/Code/Core/Structs/STeleportPointPair` _array_element)))
      (elif (== (`.Second_5_44C94781437593443EC271BAB9188421` (break `/Game/Code/Core/Structs/STeleportPointPair` _array_element)) self)
        (set `self.StreamNameThis` (`.SecondStreamName_13_FC1ED26F4C2318AF77202B8F3E32B5BD` (break `/Game/Code/Core/Structs/STeleportPointPair` _array_element)))
        (set `self.StreamNameOther` (`.FirstStramName_12_130BD56F47F345A8F33F9DB0E82DF619` (break `/Game/Code/Core/Structs/STeleportPointPair` _array_element)))
        (set `self.OtherPoint` (break `/Game/Code/Core/Structs/STeleportPointPair` _array_element))))))

(event `self.ReceiveActorBeginOverlap`
  (params (OtherActor :type "Actor Object Reference"))
  (bind _otherpoint (`self.OtherPoint`))
  (bind _returnvalue (`KismetMathLibrary.ComposeRotators` (`self.K2_GetActorRotation` _otherpoint) (struct :`Yaw` 180.0)))
  (if (== OtherActor (`GameplayStatics.GetPlayerPawn` 0))
    (`GameplayStatics.LoadStreamLevel` (`self.StreamNameOther`) true)
    (`self.K2_TeleportTo` OtherActor (+ (`self.K2_GetActorLocation` _otherpoint) (* (`KismetMathLibrary.GetForwardVector` _returnvalue) 200.0)) _returnvalue)))

(event `self.ReceiveActorEndOverlap`
  (params (OtherActor :type "Actor Object Reference"))
  (if (== OtherActor (`GameplayStatics.GetPlayerPawn` 0))
    (`GameplayStatics.UnloadStreamLevel` (`self.StreamNameThis`))))

(fn `UserConstructionScript`)