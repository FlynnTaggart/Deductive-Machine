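; BP_Clue is a clue actor for a VR investigation system that can be investigated by touch or look.
; An enabling trigger sets whether it is active, and touch and look trigger overlaps check IsTouch or IsLook, meant to test interaction type and enabled state.
; Investigation fires once through a DoOnce, marking the clue investigated and calling the clue-investigated event.
; The player's VR camera is cached at BeginPlay but not used in these graphs.
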(event `self.ReceiveBeginPlay`
  ;[1 1 1] Get VR camera
  (bind _asbp_vrcharacter (cast `/Game/Code/Core/Player/BP_VRCharacter` (`GameplayStatics.GetPlayerPawn` 0)))
  (set `self.VRCamera` (`/Game/Code/Core/Player/BP_VRCharacter.Camera` _asbp_vrcharacter)))

(event `EventEnvestigating`
  ;[1 1 1] Investigation
  (`/Engine/EditorBlueprintResources/StandardMacros.DoOnce` false
    (:`Completed`
      (set `self.bInvestigated` true)
      (`self.EventClueInvestigated`))))

(event `self.TouchTrigger.OnComponentBeginOverlap`
  (params (OverlappedComponent :type "PrimitiveComponent Object Reference") (OtherActor :type "Actor Object Reference") (OtherComp :type "PrimitiveComponent Object Reference") (OtherBodyIndex :type Integer) (bFromSweep :type Boolean) (SweepResult :type "HitResult Structure (by ref)"))
  ;[1 1 1] Touch investigation
  (if (and (`|EnumEquality` (`self.InteractionType`) "NewEnumerator4") (`self.bEnabled`))
    (`self.EventEnvestigating`)))

(event `self.LookTrigger.OnComponentBeginOverlap`
  (params (OverlappedComponent :type "PrimitiveComponent Object Reference") (OtherActor :type "Actor Object Reference") (OtherComp :type "PrimitiveComponent Object Reference") (OtherBodyIndex :type Integer) (bFromSweep :type Boolean) (SweepResult :type "HitResult Structure (by ref)"))
  ;[1 1 1] Look investigation
  (if (and (`|EnumEquality` (`self.InteractionType`) "NewEnumerator3") (`self.bEnabled`))
    (`self.EventEnvestigating`)))

(event `self.EnablingTrigger.OnComponentBeginOverlap`
  (params (OverlappedComponent :type "PrimitiveComponent Object Reference") (OtherActor :type "Actor Object Reference") (OtherComp :type "PrimitiveComponent Object Reference") (OtherBodyIndex :type Integer) (bFromSweep :type Boolean) (SweepResult :type "HitResult Structure (by ref)"))
  ;[1 1 1] Activation
  (set `self.bEnabled` true))

(event `self.EnablingTrigger.OnComponentEndOverlap`
  (params (OverlappedComponent :type "PrimitiveComponent Object Reference") (OtherActor :type "Actor Object Reference") (OtherComp :type "PrimitiveComponent Object Reference") (OtherBodyIndex :type Integer))
  ;[1 1 1] Activation
  (set `self.bEnabled` false))

(fn `UserConstructionScript`)