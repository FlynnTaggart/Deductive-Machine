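; BP_CaseScene is the investigation puzzle controller that closes a case once the player orders its Acts correctly.
; On BeginPlay it subscribes to each Act's player-order update, then checks every Act's PlayerOrder against its one-based array position.
; A full match makes all Acts non-orderable and fires EventCaseClosed, which currently only prints a debug message once.
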(event `self.ReceiveBeginPlay`
  (for _array_element (`self.Acts`)
    (add `/Game/Code/Core/InvestigationSystem/BP_Act.EventPlayerOrderUpdated` _array_element (delegate `OnActOrderSet`))))

(event `OnActOrderSet`
  (bind _result (`self.IsActsInCorrectOrder`))
  (if _result
    (for _array_element (`self.Acts`)
      (set `/Game/Code/Core/InvestigationSystem/BP_Act.bOrderable` false _array_element))
    (`self.EventCaseClosed`)))

(event `EventCaseClosed`
  (`/Engine/EditorBlueprintResources/StandardMacros.DoOnce` false
    (:`Completed`
      (`KismetSystemLibrary.PrintString` "CASE CLOSED CASE CLOSED CASE CLOSED CASE CLOSEDCASE CLOSED" true true (struct :`R` 1.0 :`G` 0.022775 :`B` 0.110439 :`A` 1.0) 110.0))))

(fn `IsActsInCorrectOrder`
  (returns (Result :type Boolean))
  (locals (Res :type Boolean))
  (set `local.Res` true)
  (for (_array_element _array_index) (`self.Acts`)
    (bind (_data_selfactor _data_name _data_clues _data_description _data_borderable _data_playerorder) (break `/Game/Code/Core/Structs/SAct` (`/Game/Code/Core/InvestigationSystem/BP_Act.Data` _array_element)))
    (set `local.Res` (and (`local.Res`) (== _data_playerorder (+ _array_index 1)))))
  (return (`local.Res`)))

(fn `UserConstructionScript`)