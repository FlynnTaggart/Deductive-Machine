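; BP_Act is an investigation act that reveals a hologram mesh once all of its clues have been investigated.
; It hides HoloMesh at BeginPlay and binds to each clue's investigated event, re-checking every clue's Investigated flag whenever one fires.
; A separate EventSetPlayerOrderId event resets Order to zero and calls EventSetOrderId.
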(event `self.ReceiveBeginPlay`
  (`SceneComponent.SetVisibility` (`self.HoloMesh`) false true)
  (for _array_element (`self.Clues`)
    (add `/Game/Code/Core/InvestigationSystem/BP_Clue.EventClueInvestigated` _array_element (delegate `OnClueInvestigated`))))

(event `OnClueInvestigated`
  (bind _result (`self.IsAllCluesInvestigated`))
  (if _result
    (`SceneComponent.SetVisibility` (`self.HoloMesh`) true true)))

(event `EventSetPlayerOrderId`
  (set `self.Order` 0)
  (`self.EventSetOrderId`))

(fn `IsAllCluesInvestigated`
  (returns (Result :type Boolean))
  (locals (bResult :type Boolean))
  (set `local.bResult` true)
  (for _array_element (`self.Clues`)
    (set `local.bResult` (and (`/Game/Code/Core/InvestigationSystem/BP_Clue.bInvestigated` _array_element) (`local.bResult`))))
  (return (`local.bResult`)))

(fn `UserConstructionScript`)