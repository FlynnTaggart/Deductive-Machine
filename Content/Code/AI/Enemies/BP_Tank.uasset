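; BP_Tank is an enemy tank Blueprint that orients its parts separately for aim and movement.
; After running the parent Tick, it sets Sphere0's world rotation to the control rotation every frame, so that part follows the controller like a turret.
; While the tank is moving, the Scene component smoothly interpolates toward the velocity direction using RInterpTo, and it holds its last rotation when stopped.
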(event `self.ReceiveTick`
  (params (DeltaSeconds :type "Float (single-precision)"))
  (bind _velocity (`MovementComponent.Velocity` (`self.CharacterMovement`)))
  (`parent.ReceiveTick` DeltaSeconds)
  (`SceneComponent.K2_SetWorldRotation` (`self.Sphere_0`) (`self.GetControlRotation`) false false)
  (if (`KismetMathLibrary.NotEqualExactly_VectorVector` _velocity)
    (`SceneComponent.K2_SetWorldRotation` (`self.Scene`) (`KismetMathLibrary.RInterpTo` (`SceneComponent.K2_GetComponentRotation` (`self.Scene`)) (`KismetMathLibrary.MakeRotFromX` _velocity) (`GameplayStatics.GetWorldDeltaSeconds`) 10.0) false false)))

(fn `UserConstructionScript`)