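; Base AI controller that turns and optionally moves its pawn toward a desired forward and location set through events.
; Sight perception writes the Blackboard TargetActor, and SetState picks the Inspection or Alerted rotation speed.
; Each tick steers by placing a spawned focus pawn far along an interpolated direction, with speed scaled by inverse remaining difference and clamped.
; Movable pawns use MoveToLocation, and debug arrows and a sphere show headings and destination.
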(event OnTargetPerceptionUpdated(AIPerception)
  (params (Actor :type Actor%20Object%20Reference) (Stimulus :type AI%20Stimulus%20Structure))
  ;[1 1 1] Sence actor
  (bind _returnvalue (Class|AIPerceptionSystem|GetSenseClassforStimulus Stimulus))
  (if (== _returnvalue "/Script/AIModule.AISense_Sight")
    (AI|Components|Blackboard|SetValueasObject (Variables|Default|GetBlackboard) (Utilities|Name|MakeLiteralName "TargetActor") (select (.bSuccessfullySensed (Utilities|Struct|BreakAIStimulus Stimulus)) Actor 0))))

(event EventSetDesiredForward
  (params (NewDesiredFwd :type Vector :default "0, 0, 0"))
  ;[1 1 1] Rotate controlled pawn towards desired forward vector and move it to desired location
  (Variables|Default|SetDesiredForward NewDesiredFwd))

(event EventTick
  (params (DeltaSeconds :type Float%20%28single-precision%29))
  ;[1 1 1] Rotate controlled pawn towards desired forward vector and move it to desired location
  (Variables|Default|SetDeltaTime DeltaSeconds)
  (|DrawDebug true)
  (CallFunction|RotateTowardsDesiredForward)
  (if (Variables|Default|GetbMovable)
    (CallFunction|MoveTowardsDesiredLoc)))

(event EventSetState
  (params (NewState :type E_AiState%20Enum :default "NewEnumerator0"))
  ;[1 1 1] Set state by BPI
  (Variables|Default|SetState NewState)
  ;[1 1 1] Set rotation speed by state
  (Variables|Default|SetRotationSpeed (Utilities|Select :Index (Variables|Default|GetState) :NewEnumerator0 (Variables|Default|GetInspectionRotSpeed) :NewEnumerator1 (Variables|Default|GetAlertedRotSpeed))))

(event EventBeginPlay
  (bind _returnvalue (Game|SpawnActorfromClass "/Game/Code/AI/Brain/BP_FocusPawn.BP_FocusPawn_C" (Math|Transform|MakeTransform "0, 0, 0" "0, 0, 0" "1,1,1") "Undefined" 0 (Pawn|GetControlledPawn)))
  (bind _output_get (Variables|Default|SetFocusActor _returnvalue))
  (AI|SetFocus _output_get))

(event EventSetDesiredLocation
  (params (DesiredLocation :type Vector :default "0, 0, 0"))
  ;[1 1 1] Rotate controlled pawn towards desired forward vector and move it to desired location
  (Variables|Default|SetDesiredLocation DesiredLocation))

(fn ConstructionScript)

(fn RotateTowardsDesiredForward
  (bind _returnvalue (Pawn|GetControlRotation :!class /Script/Engine.Controller))
  (bind _returnvalue_2 (Math|Vector|GetForwardVector _returnvalue))
  (if (Utilities|IsNeedRotation)
    (Transformation|SetActorLocation (Variables|Default|GetFocusActor) (Utilities|AddScaledDirection (Transformation|GetActorLocation (Pawn|GetControlledPawn)) (Math|Vector|Normalize (Math|Interpolation|VInterpTo _returnvalue_2 (Variables|Default|GetDesiredForward) (Variables|Default|GetDeltaTime) (Math|Float|Clamp(Float) (|((one/distance)*{F1E9990E-444E-A32D-FD3B-CAA1792C63A6}) 1.0 (Math|Vector|Distance(Vector) _returnvalue_2 (Variables|Default|GetDesiredForward))) 0.0 15.0))) 1e+04) false true)))

(fn MoveTowardsDesiredLoc
  (if (Utilities|IsNeedMovement)
    (AI|Navigation|MovetoLocation (Variables|Default|GetDesiredLocation) -1.0 true true false true 0)))

(fn GetFlightHeight
  (return 0.0))