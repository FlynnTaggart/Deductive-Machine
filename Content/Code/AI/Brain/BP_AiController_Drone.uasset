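; AI controller for a drone that runs the BT_Drone behavior tree and holds a flight-height-based desired location.
; On BeginPlay it sets that location above the pawn by FlightHeight and seeds the TargetLocation blackboard key with the pawn's position.
; MoveTowardsDesiredLoc feeds movement input toward that point, gated by IsNeedMovement, whose distance check is left unconnected.
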(event `self.ReceiveBeginPlay`
  (`parent.ReceiveBeginPlay`)
  (set `self.DesiredLocation` (`/Game/Code/Core/FunctionLibrary/BPML_VectorAlgebra.AddScaledDirection` (`self.K2_GetActorLocation` (`self.K2_GetPawn`)) (0.0 0.0 1.0) (`self.FlightHeight`)))
  (`self.RunBehaviorTree` "/Game/Code/AI/Brain/BT_Drone.BT_Drone")
  (`BlackboardComponent.SetValueAsVector` (`self.Blackboard`) "TargetLocation" (`self.K2_GetActorLocation` (`self.K2_GetPawn`))))

(fn `GetFlightHeight`
  (returns (Height :type "Float (double-precision)"))
  (return (`self.FlightHeight`)))

(fn `MoveTowardsDesiredLoc`
  (if (`self.IsNeedMovement`)
    (`Pawn.AddMovementInput` (`self.K2_GetPawn`) (`/Game/Code/Core/FunctionLibrary/BPML_VectorAlgebra.GetDirectionByPoints` (`self.K2_GetActorLocation` (`self.K2_GetPawn`)) (`self.DesiredLocation`)) 1.0 false)))

(fn `UserConstructionScript`
  (`parent.UserConstructionScript`))